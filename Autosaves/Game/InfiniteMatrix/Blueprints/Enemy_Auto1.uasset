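; Enemy actor for InfiniteMatrix, a short-lived cone hazard that damages the player on contact.
; It destroys itself four seconds after BeginPlay, or sooner when the Cone component registers a hit.
; Any hit calls TakeDamage on player 0's BP_Player without checking what was struck, as the branch condition is constant true.
; A RandomEnemy function applies a random local position offset but is not called within this Blueprint.
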(event OnComponentHit(Cone)
  (params (HitComponent :type Primitive%20Component%20Object%20Reference) (OtherActor :type Actor%20Object%20Reference) (OtherComp :type Primitive%20Component%20Object%20Reference) (NormalImpulse :type Vector :default "0, 0, 0") (Hit :type Hit%20Result%20Structure%20%28by%20ref%29))
  (if true
    (bind _asbp_player (Utilities|Casting|CastToBP_Player (Game|Player|GetPlayerPawn 0)))
    (Default|TakeDamage _asbp_player)
    (Actor|DestroyActor)
    (elif true
      _)))

(event EventBeginPlay
  (Utilities|FlowControl|Delay 4.0)
  (Actor|DestroyActor))

(event Collision|EventActorBeginOverlap
  (params (OtherActor :type Actor%20Object%20Reference)))

(event EventTick
  (params (DeltaSeconds :type Float%20%28single-precision%29)))

(fn ConstructionScript)

(fn RandomEnemy
  (bind _returnvalue (Math|Random|RandomFloatinRange 0.0 3e+02))
  (Transformation|AddActorLocalOffset (Math|Vector|MakeVector (Math|Random|RandomFloatinRange 5e+02 2e+03) _returnvalue _returnvalue) false false))