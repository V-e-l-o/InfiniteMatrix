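; Health pickup actor that restores the player's health on contact and removes itself four seconds after spawning.
; A mesh hit on BP_Player calls RegenHealth, disables the mesh collision and destroys the pack, while any hit on the HealthDestroy component destroys it without healing.
; RandomHealthpack shifts the actor by one of five preset local offsets, though nothing in this Blueprint calls it.
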(event OnComponentHit(HealthPackMesh)
  (params (HitComponent :type Primitive%20Component%20Object%20Reference) (OtherActor :type Actor%20Object%20Reference) (OtherComp :type Primitive%20Component%20Object%20Reference) (NormalImpulse :type Vector :default "0, 0, 0") (Hit :type Hit%20Result%20Structure%20%28by%20ref%29))
  (bind _asbp_player (Utilities|Casting|CastToBP_Player OtherActor))
  (Default|RegenHealth _asbp_player)
  (Collision|SetCollisionEnabled (Variables|Default|GetHealthPackMesh) "NoCollision")
  (Actor|DestroyActor))

(event OnComponentHit(HealthDestroy)
  (params (HitComponent :type Primitive%20Component%20Object%20Reference) (OtherActor :type Actor%20Object%20Reference) (OtherComp :type Primitive%20Component%20Object%20Reference) (NormalImpulse :type Vector :default "0, 0, 0") (Hit :type Hit%20Result%20Structure%20%28by%20ref%29))
  (Actor|DestroyActor))

(event EventBeginPlay
  (Utilities|FlowControl|Delay 4.0)
  (Actor|DestroyActor))

(event Collision|EventActorBeginOverlap
  (params (OtherActor :type Actor%20Object%20Reference)))

(event EventTick
  (params (DeltaSeconds :type Float%20%28single-precision%29)))

(fn ConstructionScript)

(fn RandomHealthpack
  (Transformation|AddActorLocalOffset (Utilities|Select :Index (Math|Random|RandomIntegerinRange 0 4) :Option%200 "1500.000000,-200.000000,200.000000" :Option%201 "1000.000000,300.000000,300.000000" :Option%202 "700.000000,100.000000,-345.000000" :Option%203 "2000.000000,-300.000000,250.000000" :Option%204 "1200.000000,200.000000,-100.000000") false false))